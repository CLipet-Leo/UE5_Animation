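; Child character Blueprint that adds aim input and hard-landing detection to its parent, with input disabled at BeginPlay.
; IA_Aim start and completion update IsAiming and print it for debugging.
; Grounded jump presses and walking off ledges record StartingJumpZ.
; On landing, CalculateZDifference compares the drop against MaxChuteDistance to set MustRecovery, disabling input after too long a fall; nothing here re-enables it.
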(event `self.ReceiveBeginPlay`
  (`self.DisableInput` null))

(event `EnhancedInput|/Game/Input/Actions/IA_Move`
  (params (ActionValue :type "Vector2D Structure") (ElapsedSeconds :type "Float (double-precision)") (TriggeredSeconds :type "Float (double-precision)") (InputAction :type "InputAction Object Reference" :default "/Game/Input/Actions/IA_Move.IA_Move")))

(event `EnhancedInput|/Game/Personnal/Input/Actions/IA_Aim`
  (params (ActionValue :type Boolean) (ElapsedSeconds :type "Float (double-precision)") (TriggeredSeconds :type "Float (double-precision)") (InputAction :type "InputAction Object Reference" :default "/Game/Personnal/Input/Actions/IA_Aim.IA_Aim"))
  (:`Started`
    (bind _output_get (set `self.isAiming` ActionValue :!label _label))
    (`KismetSystemLibrary.PrintString` (`KismetStringLibrary.Concat_StrStr` "Aiming : " (`KismetStringLibrary.Conv_BoolToString` _output_get)) true true (struct :`G` 0.66 :`B` 1.0 :`A` 1.0) 2.0 "Aim"))
  (:`Completed`
    (goto _label)))

(event `self.OnWalkingOffLedge`
  (params (PreviousFloorImpactNormal :type "Vector Structure (by ref)") (PreviousFloorContactNormal :type "Vector Structure (by ref)") (PreviousLocation :type "Vector Structure (by ref)") (TimeDelta :type "Float (single-precision)"))
  (bind (_returnvalue_x _returnvalue_y _returnvalue_z) (`KismetMathLibrary.BreakVector` (`self.K2_GetActorLocation`)))
  (set `self.startingJumpZ` _returnvalue_z))

(event `EnhancedInput|/Game/Input/Actions/IA_Jump`
  (params (ActionValue :type Boolean) (ElapsedSeconds :type "Float (double-precision)") (TriggeredSeconds :type "Float (double-precision)") (InputAction :type "InputAction Object Reference" :default "/Game/Input/Actions/IA_Jump.IA_Jump"))
  (bind (_returnvalue_x _returnvalue_y _returnvalue_z) (`KismetMathLibrary.BreakVector` (`self.K2_GetActorLocation`)))
  (:`Started`
    (if (not (`NavMovementComponent.IsFalling` (`self.CharacterMovement`)))
      (set `self.startingJumpZ` _returnvalue_z) ; If not set the Z value
    )))

(event `self.OnLanded`
  (params (Hit :type "HitResult Structure (by ref)"))
  (bind _output_get (set `self.mustRecovery` (`self.CalculateZDifference` Hit (`self.maxChuteDistance`))))
  (if _output_get
    (`self.DisableInput` null)))

(fn `CalculateZDifference`
  (params (Hit :type "HitResult Structure (by ref)") (Threshold :type "Float (double-precision)" :default 100.0))
  (returns (IsBeyondThreshold :type Boolean))
  (return (> (- (`self.startingJumpZ`) (.z (`.Location` (`GameplayStatics.BreakHitResult` Hit)))) Threshold)))

(fn `UserConstructionScript`
  (`parent.UserConstructionScript`))